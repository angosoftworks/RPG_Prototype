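; BP_SpawnZone is a box-shaped spawn zone that supplies random points for spawning but spawns nothing itself.
; GetRandomPointInZone picks a random offset within the Box component's scaled extent and adds its world location, ignoring the box's rotation.
; IsZoneAvailable is unfinished: its check of actor count, enabled flag and cooldown is left unconnected and never runs.
; The event graph and construction script are empty.
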(fn `GetRandomPointInZone`
  (returns (Vector :type "Vector Structure"))
  (bind _box (`self.Box`))
  (bind _x (.x (`BoxComponent.GetScaledBoxExtent` _box)))
  (bind _y (.y (`BoxComponent.GetScaledBoxExtent` _box)))
  (bind _z (.z (`BoxComponent.GetScaledBoxExtent` _box)))
  (return (+ (`KismetMathLibrary.MakeVector` (`KismetMathLibrary.RandomFloatInRange` (* _x -1.0) _x) (`KismetMathLibrary.RandomFloatInRange` (* _y -1.0) _y) (`KismetMathLibrary.RandomFloatInRange` (* _z -1.0) _z)) (`SceneComponent.K2_GetComponentLocation` _box))))

(fn `IsZoneAvailable`
  (returns (IsAvailable :type Boolean)))

(fn `UserConstructionScript`)