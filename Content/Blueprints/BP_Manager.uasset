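; BP_Manager is a village manager Actor that loads PNJ (NPC) data when play begins.
; It reads every DT_PNJData row into PNJDataArray and logs name, profession, clan, traits and relations.
; Helper functions convert each relations map into struct entries and format them as text.
; SpawnAllPNJs is called afterwards but does nothing: its loop spawning BP_PNJ actors at random spawn points is disconnected.
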(event `self.ReceiveBeginPlay`
  (`KismetSystemLibrary.PrintString` "BP_Manager → Village Initialization Started")
  (`self.InitializeVillageData`)
  (`self.SpawnAllPNJs`))

(fn `ConvertMapToArray`
  (params (InputMap :type "Map of String to Integer"))
  (returns (OutputArray :type "Array of /Game/Blueprints/Struct_RelationEntry Structure"))
  (locals (TempArray :type "Array of /Game/Blueprints/Struct_RelationEntry Structure"))
  (bind _temparray (`local.TempArray`))
  (bind _keys (`BlueprintMapLibrary.Map_Keys` InputMap))
  (for _array_element _keys
    (`KismetArrayLibrary.Array_Add` _temparray (make `/Game/Blueprints/Struct_RelationEntry` _array_element (`BlueprintMapLibrary.Map_Find` InputMap _array_element))))
  (return _temparray))

(fn `FormatPNJData`
  (params (PNJDataInput :type "/Game/Blueprints/Struct_PNJData Structure"))
  (returns (FormattedName :type String) (FormattedProfession :type String) (FormattedClan :type String) (FormattedTraits :type String) (FormattedRelations :type String))
  (bind (_name _profession _clan _traits _relations) (break `/Game/Blueprints/Struct_PNJData` PNJDataInput))
  (bind (_ambition `_loyauté` `_sociabilité`) (break `/Game/Blueprints/Struct_PNJTraits` _traits))
  (bind _outputarray (`self.ConvertMapToArray` _relations))
  (bind _formattedrelationsstring (`self.FormatRelationsArray` _outputarray))
  (return _name _profession _clan (`KismetTextLibrary.Conv_TextToString` (`|FormatText` "Ambition = {Ambition}, Loyauté = {Loyauté}, Sociabilité = {Sociabilité}" _ambition `_loyauté` `_sociabilité`)) _formattedrelationsstring))

(fn `FormatRelationsArray`
  (params (RelationsArray :type "Array of /Game/Blueprints/Struct_RelationEntry Structure"))
  (returns (FormattedRelationsString :type String))
  (locals (CurrentRelationsString :type String))
  (set `local.CurrentRelationsString` "")
  (for _array_element RelationsArray
    (bind (_relationname _relationscore) (break `/Game/Blueprints/Struct_RelationEntry` _array_element))
    (bind _output_get (set `local.CurrentRelationsString` (`KismetStringLibrary.Concat_StrStr` (stale _output_get) (`KismetTextLibrary.Conv_TextToString` (`|FormatText` "{NomRelation} : {Score} |" _relationname _relationscore))))))
  (return (`local.CurrentRelationsString`)))

(fn `InitializeVillageData`
  (`self.LoadPNJData`))

(fn `LoadPNJData`
  (bind _outrownames (`DataTableFunctionLibrary.GetDataTableRowNames` "/Game/Data/DT_PNJData.DT_PNJData"))
  (for _array_element _outrownames
    (bind _returnvalue (`|GetDataTableRow` "/Game/Data/DT_PNJData.DT_PNJData" _array_element)
      (:`then`
        (bind (_formattedname _formattedprofession _formattedclan _formattedtraits _formattedrelations) (`self.FormatPNJData` _returnvalue))
        (`KismetSystemLibrary.PrintString` (`KismetStringLibrary.Concat_StrStr` "Nom :" _formattedname " Métier :" _formattedprofession " Clan :" _formattedclan " Traits :" _formattedtraits " Relations :" _formattedrelations))
        (`KismetArrayLibrary.Array_Add` (`self.PNJDataArray`))))))

(fn `SpawnAllPNJs`)

(fn `UserConstructionScript`)