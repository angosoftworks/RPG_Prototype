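; BP_SpawnManager is a manager that spawns actors at random points in BP_SpawnZone actors, with its event graph left empty.
; InitializeSpawnZones caches the zones, and StartSpawnLoop runs SpawnActor on a looping timer.
; SpawnActor only spawns once the tracked count is at or above MaxSpawnedActors, which looks inverted.
; RecycleActor deactivates actors into a pool that SpawnActor never reuses, and SpawnActor also bypasses GetAvailableZone.
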(fn `GetAvailableZone`
  (returns (AvailableZone :type "/Game/Blueprints/BP_SpawnZone Object Reference"))
  (bind _outactors (`GameplayStatics.GetAllActorsOfClass` "/Game/Blueprints/BP_SpawnZone.BP_SpawnZone_C"))
  (for _array_element _outactors
    (if (`/Game/Blueprints/BP_SpawnZone.IsZoneAvailable` _array_element)
      (return _array_element))))

(fn `InitializeSpawnZones`
  (bind _outactors (`GameplayStatics.GetAllActorsOfClass` "/Game/Blueprints/BP_SpawnZone.BP_SpawnZone_C"))
  (set `self.SpawnZones` _outactors))

(fn `RecycleActor`
  (params (ActorToRecycle :type "Actor Object Reference"))
  (`self.SetActorHiddenInGame` ActorToRecycle true)
  (`self.SetActorEnableCollision` ActorToRecycle false)
  (`self.SetActorTickEnabled` ActorToRecycle false)
  (`KismetArrayLibrary.Array_Add` (`self.ActorPool`) ActorToRecycle))

(fn `SpawnActor`
  (if (>= (`KismetArrayLibrary.Array_Length` (`self.SpawnedActors`)) (`self.MaxSpawnedActors`))
    (bind _vector (`/Game/Blueprints/BP_SpawnZone.GetRandomPointInZone` (`KismetArrayLibrary.Array_Random` (`self.SpawnZones`))))
    (bind _returnvalue (`|SpawnActorFromClass` (`self.ActorToSpawn`) (`KismetMathLibrary.Conv_VectorToTransform` _vector) "AdjustIfPossibleButAlwaysSpawn" "MultiplyWithRoot" null null))
    (`KismetArrayLibrary.Array_Add` (`self.SpawnedActors`) _returnvalue)))

(fn `StartSpawnLoop`
  (if (> (`KismetArrayLibrary.Array_Length` (`self.SpawnZones`)) 0)
    (`KismetSystemLibrary.K2_SetTimer` null "SpawnActor" (`self.SpawnInterval`) true)
    (else
      (`KismetSystemLibrary.PrintString` "No Spawn Zones! Check Initialize"))))

(fn `UserConstructionScript`)